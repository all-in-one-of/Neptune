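; Player controller that routes all player input to the possessed Player_BP pawn.
; On BeginPlay it casts and caches the controlled pawn, then forwards look, movement, sprint, lean, crouch, multi-jump and visor sweep inputs to its functions.
; Weapon inputs drive fire, aim and cycling on the pawn, while reload calls the current weapon directly.
; Weapon selection derives a zero-based slot index from the pressed key's display name.
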(event EventBeginPlay
  ;[0.1612 0.6508 1] Init player reference
  (bind _asplayer_bp (Utilities|Casting|CastToPlayer_BP (Pawn|GetControlledPawn)))
  (Variables|Default|SetMy%20Player _asplayer_bp))

(event Input|ActionEvents|InputActionJump
  (params (Key :type Key%20Structure))
  ;[1 1 1] Locomotion handling
  (:Pressed
    (Default|DoMultiJump (Variables|Default|GetMy%20Player))))

(event Input|ActionEvents|InputActionAbilityUp
  (params (Key :type Key%20Structure))
  ;[0.152 0.6067 1] Ability handling
  (:Pressed
    (Default|VisorSweep (Variables|Default|GetMy%20Player))))

(event Input|ActionEvents|InputActionCrouch
  (params (Key :type Key%20Structure))
  ;[1 1 1] Locomotion handling
  (:Pressed
    (Default|ToggleCrouch (Variables|Default|GetMy%20Player))))

(event Input|ActionEvents|InputActionReload
  (params (Key :type Key%20Structure))
  ;[0.6798 0.1602 1] Weapon handling
  (:Pressed
    (Default|Reload (.Weapon (Default|GetCurrentWeapon (Variables|Default|GetMy%20Player))))))

(event Input|ActionEvents|InputActionLean
  (params (Key :type Key%20Structure))
  (bind _my_player (Variables|Default|GetMy%20Player))
  ;[1 1 1] Locomotion handling
  (:Pressed
    (Default|StartLeaning _my_player))
  (:Released
    (Default|StopLeaning _my_player)))

(event Input|ActionEvents|InputActionSelectWeapon
  (params (Key :type Key%20Structure))
  ;[0.6798 0.1602 1] Weapon handling
  (:Pressed
    (Default|SetWeapon (Variables|Default|GetMy%20Player) (- (Math|Conversions|ToInteger(Byte) (Utilities|String|ToString(Text) (Class|KismetInputLibrary|KeyGetDisplayName Key))) 1))))

(event Input|ActionEvents|InputActionHoldSprint
  (params (Key :type Key%20Structure))
  (bind _my_player (Variables|Default|GetMy%20Player))
  ;[1 0.7271 0.04911] Sprint handling
  (:Pressed
    (Default|StartSprinting _my_player))
  (:Released
    (Default|StopSprinting _my_player)))

(event Input|ActionEvents|InputActionToggleSprint
  (params (Key :type Key%20Structure))
  ;[1 0.7271 0.04911] Sprint handling
  (:Pressed
    (Default|ToggleSprinting (Variables|Default|GetMy%20Player))))

(event Input|AxisEvents|InputAxisMoveForward
  (params (AxisValue :type Float%20%28single-precision%29))
  ;[1 1 1] Locomotion handling
  (Default|MoveForward (Variables|Default|GetMy%20Player) AxisValue))

(event Input|AxisEvents|InputAxisMoveRight
  (params (AxisValue :type Float%20%28single-precision%29))
  ;[1 1 1] Locomotion handling
  (Default|MoveRight (Variables|Default|GetMy%20Player) AxisValue))

(event Input|AxisEvents|InputAxisLookRight
  (params (AxisValue :type Float%20%28single-precision%29))
  ;[1 0.09604 0] Camera handling
  (Default|LookRight (Variables|Default|GetMy%20Player) AxisValue))

(event Input|AxisEvents|InputAxisLookUp
  (params (AxisValue :type Float%20%28single-precision%29))
  ;[1 0.09604 0] Camera handling
  (Default|LookUp (Variables|Default|GetMy%20Player) AxisValue))

(event Input|AxisEvents|InputAxisAim
  (params (AxisValue :type Float%20%28single-precision%29))
  ;[0.6798 0.1602 1] Weapon handling
  (Default|Aim (Variables|Default|GetMy%20Player) AxisValue))

(event Input|AxisEvents|InputAxisFire
  (params (AxisValue :type Float%20%28single-precision%29))
  ;[0.6798 0.1602 1] Weapon handling
  (Default|Fire (Variables|Default|GetMy%20Player) AxisValue))

(event Input|AxisEvents|InputAxisCycleWeapons
  (params (AxisValue :type Float%20%28single-precision%29))
  ;[0.6798 0.1602 1] Weapon handling
  (Default|CycleWeapons (Variables|Default|GetMy%20Player) AxisValue))

(fn ConstructionScript)