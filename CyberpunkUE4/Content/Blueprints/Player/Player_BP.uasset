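; First-person player character with multi-jump, sprint, crouch, leaning, camera effects and component-based weapons.
; BeginPlay creates the HUD, then it and Tick run raycast, locomotion, camera and weapon handling in sequence.
; A forward sphere trace detects obstructions, swinging the gun aside and blocking fire and aim.
; Timelines and interpolated values drive capsule crouch, landing dip, FOV, view bob, roll and lean, while the current Weapon_BPC supplies aim and recoil.
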(event EventBeginPlay
  (Utilities|FlowControl|Sequence
    (:then_0
      ;[0.2083 0.2432 1] Init HUD
      (bind _returnvalue (UserInterface|CreateWidget "/Game/UI/HUD_UMG.HUD_UMG_C" (Game|GetPlayerController 0)))
      (bind _output_get (Variables|UI|SetHUD _returnvalue))
      (UserInterface|Viewport|AddtoViewport _output_get 0))
    (:then_1
      (Utilities|FlowControl|Sequence
        (:then_0
          (|RaycastHandling (stale EventTick DeltaSeconds)) ; enters at EventBeginPlay
        )
        (:then_1
          (|LocomotionHandling (stale EventTick DeltaSeconds)) ; enters at EventBeginPlay
        )
        (:then_2
          (|CameraHandling (stale EventTick DeltaSeconds)) ; enters at EventBeginPlay
        )
        (:then_3
          (|WeaponHandling (stale EventTick DeltaSeconds)) ; enters at EventBeginPlay
        )))))

(event EventTick
  (params (DeltaSeconds :type Float%20%28single-precision%29))
  (Utilities|FlowControl|Sequence
    (:then_0
      (|RaycastHandling DeltaSeconds))
    (:then_1
      (|LocomotionHandling DeltaSeconds))
    (:then_2
      (|CameraHandling DeltaSeconds))
    (:then_3
      (|WeaponHandling DeltaSeconds))))

(fn ConstructionScript
  (Utilities|FlowControl|Sequence
    (:then_0
      (for _array_element (Actor|GetComponentsByClass "/Script/Engine.PostProcessComponent")
        (CallFunction|SetPostProcessBlendWeight _array_element (Math|Conversions|ToFloat(Boolean) (Variables|Default|GetPreview%20Post%20Process)))))
    (:then_1
      (bind _output_get (Variables|Weapon|SetWeapons (Actor|GetComponentsByClass "/Game/Blueprints/Components/Weapon_BPC.Weapon_BPC_C")))
      (for _array_element_2 _output_get
        (Default|Initialize _array_element_2 (Variables|Weapon|GetWeaponMesh))))))

(fn GetCamera
  (bind _camera (Variables|Camera|GetCamera))
  (return (Variables|Camera|GetCameraPivot) _camera (Transformation|GetWorldLocation _camera) (Math|Vector|GetForwardVector _camera) (Math|Vector|GetRightVector _camera)))

(fn GetMovementSpeed
  (bind _sprint_multiplier (Variables|Locomotion|Sprint|GetSprint%20Multiplier))
  (bind _cached_walk_speed (Variables|Locomotion|Movement|GetCached%20Walk%20Speed))
  (bind _returnvalue (* _cached_walk_speed _sprint_multiplier))
  (return (Math|Float|SelectFloat _returnvalue _cached_walk_speed (Variables|Locomotion|Sprint|GetIs%20Sprinting)) _cached_walk_speed _returnvalue))

(fn SetPostProcessBlendWeight
  (params (Target :type Post%20Process%20Component%20Object%20Reference) (BlendWeight :type Float%20%28single-precision%29))
  (bind _output_get (Variables|/Script/Engine.PostProcessComponent|SetBlendWeight Target BlendWeight))
  (Variables|/Script/Engine.PostProcessComponent|SetbEnabled Target (> _output_get 0.0)))

(fn LerpFOV
  (params (FOV :type Float%20%28single-precision%29) (Alpha :type Float%20%28single-precision%29))
  (Camera|SetFieldOfView (Variables|Camera|GetCamera) (Math|Float|Lerp (Variables|Camera|GetCached%20FOV) FOV Alpha)))

(fn LerpFOVMultiplier
  (params (FOV%20Multiplier :type Float%20%28single-precision%29) (Alpha :type Float%20%28single-precision%29))
  (Camera|LerpFOV (* (Variables|Camera|GetCached%20FOV) FOV%20Multiplier) Alpha))

(fn GetCurrentWeapon
  (return (Utilities|Array|Get(acopy) (Variables|Weapon|GetWeapons) (Variables|Weapon|GetCurrent%20Weapon%20Index))))

(fn IsLeaning
  (return (>= (Variables|Weapon|Lean|GetLean) 0.2)))

(event Custom|StartCrouching
  (bind _capsulecomponent (Variables|Collision|GetCapsuleComponent))
  ;[1 0.04459 0] Crouching
  (Variables|Locomotion|Crouch|SetIs%20Crouching true)
  (bind _crouch (Timeline|Crouch%20Animation Play)
    (:Update
      (Components|Capsule|SetCapsuleRadius _capsulecomponent (Math|Float|Lerp (Variables|Locomotion|Crouch|GetCached%20Capsule%20Radius) (Variables|Locomotion|Crouch|GetCrouch%20Capsule%20Radius) _crouch) false)
      (Components|Capsule|SetCapsuleHalfHeight _capsulecomponent (Math|Float|Lerp (Variables|Locomotion|Crouch|GetCached%20Capsule%20Half%20Height) (Variables|Locomotion|Crouch|GetCrouch%20Capsule%20Half%20Height) _crouch) true))
    (:Finished
      (Utilities|FlowControl|DoOnce false) ; enters at Reset
    )))

(event Custom|StopCrouching
  (bind _capsulecomponent (Variables|Collision|GetCapsuleComponent))
  ;[1 0.04459 0] Crouching
  (Variables|Locomotion|Crouch|SetIs%20Crouching false)
  (bind _crouch (Timeline|Crouch%20Animation Reverse)
    (:Update
      (Components|Capsule|SetCapsuleRadius _capsulecomponent (Math|Float|Lerp (Variables|Locomotion|Crouch|GetCached%20Capsule%20Radius) (Variables|Locomotion|Crouch|GetCrouch%20Capsule%20Radius) _crouch) false)
      (Components|Capsule|SetCapsuleHalfHeight _capsulecomponent (Math|Float|Lerp (Variables|Locomotion|Crouch|GetCached%20Capsule%20Half%20Height) (Variables|Locomotion|Crouch|GetCrouch%20Capsule%20Half%20Height) _crouch) true))
    (:Finished
      (Utilities|FlowControl|DoOnce false) ; enters at Reset
    )))

(event Custom|ToggleCrouch
  ;[1 0.04459 0] Crouching
  (Utilities|FlowControl|DoOnce false
    (:Completed
      (if (Variables|Locomotion|Crouch|GetIs%20Crouching)
        (CallFunction|StopCrouching)
        (else
          (Utilities|FlowControl|Sequence
            (:then_0
              (CallFunction|StartCrouching))
            (:then_1
              (if (Variables|Locomotion|Sprint|GetIs%20Sprinting) ; stop sprinting if crouching
                (CallFunction|StopSprinting) ; add slide to this
              ))))))))

(event Custom|DoMultiJump
  (bind _jump_count (Variables|Locomotion|Jump|GetJump%20Count))
  ;[1 0.7389 0.2091] Multi jump
  (Variables|Locomotion|Jump|SetIs%20Jumping true)
  (bind _counter (Utilities|FlowControl|DoN _jump_count)
    (:Exit
      (Character|LaunchCharacter (Math|Vector|MakeVector 0.0 0.0 (* (Variables|/Script/Engine.CharacterMovementComponent|GetJumpZVelocity (Variables|Character|GetCharacterMovement)) (CallFunction|OneMinus (CallFunction|IntFloatDivision (- _counter 1) _jump_count)))) false false))))

(event Custom|StopSprinting
  ;[0.5206 0.3632 1] Sprint
  (Variables|Locomotion|Sprint|SetIs%20Sprinting false)
  (Variables|/Script/Engine.CharacterMovementComponent|SetMaxWalkSpeed (Variables|Character|GetCharacterMovement) (.Max%20Walk%20Speed (Locomotion|Sprint|GetMovementSpeed)))
  ;[0.282 1 0.1106] FOV animation
  (bind _fov (Timeline|Sprint%20FOV%20Animation Reverse)
    (:Update
      (Camera|LerpFOVMultiplier (Variables|Locomotion|Sprint|GetSprint%20FOV%20Multiplier) _fov)
      (CallFunction|SetPostProcessBlendWeight (Variables|Locomotion|Sprint|GetSprintPostProcess) _fov))))

(event Custom|StartSprinting
  ;[0.5206 0.3632 1] Sprint
  (if (and (>= (/ (Variables|Locomotion|Movement|GetMovement%20Velocity) (.Max%20Walk%20Speed (Locomotion|Sprint|GetMovementSpeed))) 0.25) (not (Default|IsAiming (Weapon|GetCurrentWeapon))))
    (Utilities|FlowControl|Sequence
      (:then_0
        (Variables|Locomotion|Sprint|SetIs%20Sprinting true)
        (Variables|/Script/Engine.CharacterMovementComponent|SetMaxWalkSpeed (Variables|Character|GetCharacterMovement) (.Max%20Sprint%20Speed (Locomotion|Sprint|GetMovementSpeed)))
        ;[0.282 1 0.1106] FOV animation
        (bind _fov (Timeline|Sprint%20FOV%20Animation Play)
          (:Update
            (Camera|LerpFOVMultiplier (Variables|Locomotion|Sprint|GetSprint%20FOV%20Multiplier) _fov)
            (CallFunction|SetPostProcessBlendWeight (Variables|Locomotion|Sprint|GetSprintPostProcess) _fov))))
      (:then_1
        (if (Variables|Locomotion|Crouch|GetIs%20Crouching) ; stop crouching if sprinting while crouched
          (CallFunction|StopCrouching))))))

(event Custom|MoveRight
  (params (Axis%20Value :type Float%20%28single-precision%29))
  (bind _returnvalue (Utilities|Time|GetWorldDeltaSeconds))
  (bind _returnvalue_2 (Math|Float|MakeLiteralFloat 1.0))
  ;[0.2904 1 0.5242] Movement
  (Utilities|FlowControl|Sequence
    (:then_0
      (if (Variables|Locomotion|Movement|GetCan%20Move)
        (Pawn|Input|AddMovementInput (CallFunction|VectorXY (.Camera%20Right (Locomotion|Camera|GetCamera)) 1.0) Axis%20Value false)))
    (:then_1
      (Variables|Locomotion|Movement|SetSmoothed%20Movement%20Input (Math|Vector2D|MakeVector2D (Math|Interpolation|FInterpTo (.x (Variables|Locomotion|Movement|GetSmoothed%20Movement%20Input)) Axis%20Value _returnvalue _returnvalue_2) (Math|Interpolation|FInterpTo (.y (Variables|Locomotion|Movement|GetSmoothed%20Movement%20Input)) (stale Custom|MoveForward Axis%20Value) _returnvalue _returnvalue_2))))))

(event Custom|MoveForward
  (params (Axis%20Value :type Float%20%28single-precision%29))
  (bind _returnvalue (Utilities|Time|GetWorldDeltaSeconds))
  (bind _returnvalue_2 (Math|Float|MakeLiteralFloat 1.0))
  ;[0.2904 1 0.5242] Movement
  (Utilities|FlowControl|Sequence
    (:then_0
      (if (Variables|Locomotion|Movement|GetCan%20Move)
        (Pawn|Input|AddMovementInput (CallFunction|VectorXY (.Camera%20Forward (Locomotion|Camera|GetCamera)) 1.0) Axis%20Value false)))
    (:then_1
      (Variables|Locomotion|Movement|SetSmoothed%20Movement%20Input (Math|Vector2D|MakeVector2D (Math|Interpolation|FInterpTo (.x (Variables|Locomotion|Movement|GetSmoothed%20Movement%20Input)) (stale Custom|MoveRight Axis%20Value) _returnvalue _returnvalue_2) (Math|Interpolation|FInterpTo (.y (Variables|Locomotion|Movement|GetSmoothed%20Movement%20Input)) Axis%20Value _returnvalue _returnvalue_2))))))

(event EventOnLanded
  (params (Hit :type Hit%20Result%20Structure%20%28by%20ref%29))
  (bind _returnvalue (Transformation|GetVelocity))
  (bind _jump_count (Variables|Locomotion|Jump|GetJump%20Count))
  (bind _cached_camera_pivot_offset (Variables|Camera|GetCached%20Camera%20Pivot%20Offset))
  ;[1 0.7389 0.2091] Multi jump
  (Variables|Locomotion|Jump|SetIs%20Jumping false)
  (Utilities|FlowControl|Sequence
    (:then_0
      (Utilities|FlowControl|DoN _jump_count) ; enters at Reset
    )
    (:then_1
      ;[1 0.1444 0.7439] Landing animation
      (if (<= (.z _returnvalue) (Variables|Locomotion|Jump|GetLanding%20Animation%20Gravity%20Z%20Threshold))
        (Utilities|FlowControl|DoOnce false :!label _label
          (:Completed
            (Variables|Locomotion|Jump|SetCached%20Landing%20Gravity%20Z (.z _returnvalue))
            (bind _position (Timeline|Landing%20Animation PlayFromStart)
              (:Update
                (Transformation|SetRelativeLocation (Variables|Camera|GetCameraPivot) (Math|Vector|MakeVector (.x _cached_camera_pivot_offset) (.y _cached_camera_pivot_offset) (Math|Float|Lerp (.z _cached_camera_pivot_offset) (+ (.z _cached_camera_pivot_offset) (* (Variables|Locomotion|Jump|GetLanding%20Animation%20Relative%20Z%20Offset) (CallFunction|Saturate (/ (Variables|Locomotion|Jump|GetCached%20Landing%20Gravity%20Z) -1e+03)))) _position)) false false))
              (:Finished
                (goto _label Reset)))))))))

(event Custom|LookRight
  (params (Axis%20Value :type Float%20%28single-precision%29))
  ;[1 0.09821 0.02851] Camera controls
  (Transformation|AddRelativeRotation (Variables|Camera|GetCameraPivot) (Math|Rotator|MakeRotator 0.0 0.0 (* (.x (Variables|Camera|GetTurn%20Speed)) Axis%20Value (Utilities|Time|GetWorldDeltaSeconds))) false false))

(event Custom|LookUp
  (params (Axis%20Value :type Float%20%28single-precision%29))
  ;[1 0.09821 0.02851] Camera controls
  (Transformation|AddRelativeRotation (Variables|Camera|GetCameraPivot) (Math|Rotator|MakeRotator 0.0 (* Axis%20Value (.y (Variables|Camera|GetTurn%20Speed)) (Utilities|Time|GetWorldDeltaSeconds)) 0.0) false false))

(event Custom|Aim
  (params (Axis%20Value :type Float%20%28single-precision%29))
  (bind _weapon (Weapon|GetCurrentWeapon))
  (bind _cached_interpolation_pivot_transform (Variables|Weapon|GetCached%20Interpolation%20Pivot%20Transform))
  (bind _cached_interpolate_rotation_speed (Variables|Weapon|GetCached%20Interpolate%20Rotation%20Speed))
  (bind _aim (Variables|/Game/Blueprints/Components/Weapon_BPC.Weapon_BPC_C|GetAim _weapon))
  ;[1 0.413 0.002553] Aiming
  (|SetBy-RefVar _aim (Math|Interpolation|FInterpTo _aim (* (Math|Conversions|ToFloat(Boolean) (Math|Boolean|ANDBoolean (> Axis%20Value 0.25) (not (Variables|Locomotion|Sprint|GetIs%20Sprinting)) (not (Variables|Camera|Blocking|GetIs%20Blocking)))) (CallFunction|Saturate Axis%20Value)) (Utilities|Time|GetWorldDeltaSeconds) 12.0))
  (Transformation|SetRelativeLocation (Variables|Camera|GetInterpolationPivot) (Math|Vector|Lerp(Vector) (.location _cached_interpolation_pivot_transform) (Math|Vector|MakeVector (.X (Math|Vector|BreakVector (.location _cached_interpolation_pivot_transform))) 0.0 -25.0) _aim) false false)
  (Utilities|Struct|SetmembersinFInterpolateSettings (Variables|/Game/Blueprints/Components/InterpolatedSceneComponent_BPC.InterpolatedSceneComponent_BPC_C|GetInterpolate%20Rotation (Variables|Camera|GetInterpolatedSceneComponent)) (Math|Float|Lerp _cached_interpolate_rotation_speed (* _cached_interpolate_rotation_speed 2.5) _aim))
  (Utilities|FlowControl|Sequence
    (:then_0
      (if (Default|IsAiming _weapon)
        (goto _label Open)
        (elif (<= _aim 0.0)
          (goto _label Close))))
    (:then_1
      (Utilities|FlowControl|Gate true :!label _label
        (:Exit
          (Camera|LerpFOVMultiplier 0.8 _aim))))))

(event Custom|Fire
  (params (Axis%20Value :type Float%20%28single-precision%29))
  (bind _weapon (Weapon|GetCurrentWeapon))
  ;[1 0.00718 0] Fire
  (if (>= Axis%20Value 0.5)
    (if (not (Variables|Camera|Blocking|GetIs%20Blocking)) ; no blocking then fire
      (Default|Pressfire _weapon)
      ;[1 0.8398 0] Reload if trying to fire an empty weapon
      (if (Default|IsMagazineEmpty _weapon)
        (Default|Reload _weapon))
      (else
        (Default|ReleaseFire _weapon :!label _label)))
    (else
      (goto _label))))

(event Custom|StopLeaning
  ;[0.8792 0.2916 1] Leaning
  (Variables|Locomotion|Movement|SetCan%20Move true)
  (bind _lean (Timeline|Lean%20Animation Reverse)
    (:Update
      (Variables|Weapon|Lean|SetLean _lean))))

(event Custom|StartLeaning
  ;[0.8792 0.2916 1] Leaning
  (Variables|Locomotion|Movement|SetCan%20Move false)
  (bind _lean (Timeline|Lean%20Animation Play)
    (:Update
      (Variables|Weapon|Lean|SetLean _lean))))