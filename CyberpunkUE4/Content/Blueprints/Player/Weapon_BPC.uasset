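; Player weapon component that handles fire rate, firing sound and a normalized recoil value, with no projectile or hit logic.
; Fire is gated by a DoOnce that resets after a delay derived from rounds per minute, playing sound at the owner's location as a muzzle placeholder.
; Each shot adds aim-scaled recoil plus frame delta time, clamped to 0–1.
; Tick eases recoil toward zero, scaling cooldown speed when not firing.
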(event Custom|Fire
  (bind _recoil (Variables|Stats|Recoil|GetRecoil))
  (Utilities|FlowControl|DoOnce false :!label _label
    (:Completed
      (Utilities|FlowControl|Sequence
        (:then_0
          (Variables|Default|SetIs%20Firing true)
          (Audio|PlaySoundatLocation (Variables|Sound|GetFire%20Sound) (Transformation|GetActorLocation (Components|GetOwner)) "0, 0, 0" (Variables|Sound|GetFire%20Volume) 1.0 0.0 0 0 0)
          (|SetBy-RefVar _recoil (CallFunction|Saturate (+ _recoil (CallFunction|GetRecoilRate) (Utilities|Time|GetWorldDeltaSeconds)))))
        (:then_1
          (Utilities|FlowControl|Delay (CallFunction|GetFireDelay))
          (Variables|Default|SetIs%20Firing false)
          (goto _label Reset))))))

(event EventTick
  (params (DeltaSeconds :type Float%20%28single-precision%29))
  (bind _recoil (Variables|Stats|Recoil|GetRecoil))
  ;[0.6671 1 0.3541] Recoil cooldown
  (|SetBy-RefVar _recoil (Math|Interpolation|FInterpTo _recoil 0.0 (Utilities|Time|GetWorldDeltaSeconds) (* (Variables|Stats|Recoil|GetCooldown%20Rate) (Math|Float|SelectFloat 1.0 (Variables|Stats|Recoil|GetIdle%20Cooldown%20Multiplier) (Variables|Default|GetIs%20Firing))))))

(event EventBeginPlay
  ;[1 0.1036 0] Init
  (Variables|Stats|Recoil|SetRecoil 0.0)
  (Variables|Default|SetIs%20Firing false))

(fn GetFireDelay
  (return (/ 1.0 (/ (Variables|Stats|GetRounds%20Per%20Minute) 6e+01))))

(fn IsAiming
  (return (>= (Variables|Default|GetAim) 0.05)))

(fn GetRecoilRate
  (bind _recoil_rate (Variables|Stats|Recoil|GetRecoil%20Rate))
  (return (Math|Float|Lerp _recoil_rate (* _recoil_rate (Variables|Stats|Recoil|GetAiming%20Recoil%20Multiplier)) (Variables|Default|GetAim))))