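; Ammo component that tracks a magazine and a reserve ammo pool and handles timed, cancellable reloading.
; Reload starts a timer, guarded by a DoOnce and skipped when the magazine is full or the pool empty, which fires QuickReload.
; QuickReload moves the missing rounds from pool to magazine, limited by what the pool holds.
; Clamped setters and adders broadcast dispatchers for changes, empty and full states, and reload progress.
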(event Custom|Reload
  (if (and (not (Stats|Ammo|IsMagazineFull)) (not (Stats|Ammo|IsAmmoPoolEmpty))) ; If not full
    (Utilities|FlowControl|DoOnce false
      (:Completed
        (Utilities|FlowControl|Sequence
          (:then_0
            (bind _returnvalue (Utilities|Time|SetTimerbyEvent (delegate Custom|QuickReload) (Variables|Stats|Ammo|GetReload%20Time)))
            (Variables|Stats|Ammo|SetReload%20Timer _returnvalue))
          (:then_1
            (Default|CallOnReloadTriggered)))))))

(event Custom|CancelReload
  (Utilities|FlowControl|Sequence
    (:then_0
      (Utilities|Time|ClearandInvalidateTimerbyHandle (Variables|Stats|Ammo|GetReload%20Timer)))
    (:then_1
      (Utilities|FlowControl|DoOnce false) ; enters at Reset
    )
    (:then_2
      (Default|CallOnReloadCancelled))))

(event Custom|QuickReload
  (Utilities|FlowControl|Sequence
    (:then_0
      (bind _magazine_delta (Stats|Ammo|CalculateMagazine))
      (Stats|Ammo|AddMagazine _magazine_delta)
      (Stats|Ammo|AddAmmoPool (* _magazine_delta -1)))
    (:then_1
      (Utilities|FlowControl|DoOnce false) ; enters at Reset
    )
    (:then_2
      (Default|CallOnReloadComplete))))

(fn SetAmmoPool
  (params (New%20Ammo :type Integer))
  (Utilities|FlowControl|Sequence
    (:then_0
      (Variables|Stats|Ammo|SetAmmo%20Pool (Math|Integer|Clamp(Integer) New%20Ammo 0 (Variables|Stats|Ammo|GetAmmo%20Pool%20Size))))
    (:then_1
      (Default|CallOnAmmoPoolSet))))

(fn AddAmmoPool
  (params (Delta :type Integer))
  (if (!= Delta 0)
    (Utilities|FlowControl|Sequence
      (:then_0
        (Stats|Ammo|SetAmmoPool (+ (Variables|Stats|Ammo|GetAmmo%20Pool) Delta))
        (if (Stats|Ammo|IsAmmoPoolEmpty)
          (Default|CallOnAmmoPoolEmpty)
          (elif (Stats|Ammo|IsAmmoPoolFull)
            (Default|CallOnAmmoPoolFull))))
      (:then_1
        (Default|CallOnAmmoPoolAdded)))))

(fn SetMagazine
  (params (New%20Magazine :type Integer))
  (Utilities|FlowControl|Sequence
    (:then_0
      (Variables|Stats|Ammo|SetMagazine (Math|Integer|Clamp(Integer) New%20Magazine 0 (Variables|Stats|Ammo|GetMagazine%20Size))))
    (:then_1
      (Default|CallOnMagazineSet))))

(fn IsAmmoPoolEmpty
  (return (<= (Variables|Stats|Ammo|GetAmmo%20Pool) 0)))

(fn IsMagazineEmpty
  (return (<= (Variables|Stats|Ammo|GetMagazine) 0)))

(fn IsAmmoPoolFull
  (return (>= (Variables|Stats|Ammo|GetAmmo%20Pool) (Variables|Stats|Ammo|GetAmmo%20Pool%20Size))))

(fn IsMagazineFull
  (return (>= (Variables|Stats|Ammo|GetMagazine) (Variables|Stats|Ammo|GetMagazine%20Size))))

(fn AddMagazine
  (params (Delta :type Integer))
  (if (!= Delta 0)
    (Utilities|FlowControl|Sequence
      (:then_0
        (Stats|Ammo|SetMagazine (+ (Variables|Stats|Ammo|GetMagazine) Delta))
        (if (Stats|Ammo|IsMagazineEmpty)
          (Default|CallOnMagazineEmpty)
          (elif (Stats|Ammo|IsMagazineFull)
            (Default|CallOnMagazineFull))))
      (:then_1
        (Default|CallOnMagazineAdded)))))

(fn CalculateMagazine
  (return (Math|Integer|Clamp(Integer) (- (Variables|Stats|Ammo|GetMagazine%20Size) (Variables|Stats|Ammo|GetMagazine)) 0 (Variables|Stats|Ammo|GetAmmo%20Pool))))

(fn IsReloading
  (return (Utilities|Time|IsTimerActivebyHandle (Variables|Stats|Ammo|GetReload%20Timer))))