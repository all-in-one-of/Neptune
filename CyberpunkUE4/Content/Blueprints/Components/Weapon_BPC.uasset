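; Weapon component that handles firing, fire modes, recoil and ammo use on a mesh supplied through Initialize.
; PressFire is gated by DoOnce, magazine and reload checks, then plays muzzle sound and particles, adds aim-scaled recoil and spends ammo.
; After a rounds-per-minute delay, Automatic reopens the gate, while Semi-Automatic and Burst-Fire arm a second DoOnce that ReleaseFire uses to reopen it.
; Tick interpolates recoil toward zero, with cooldown speed depending on IsFiring.
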(event Custom|PressFire
  (bind _returnvalue (Utilities|Name|MakeLiteralName "Muzzle"))
  (bind _fire_particle_system (Variables|Effects|GetFire%20Particle%20System))
  (bind _recoil (Variables|Stats|Recoil|GetRecoil))
  (bind _mesh (Variables|Default|GetMesh))
  (bind _fire_sound (Variables|Effects|GetFire%20Sound))
  (bind _returnvalue_2 (Transformation|GetSocketTransform _mesh _returnvalue "RTS_World"))
  (Utilities|FlowControl|DoOnce false :!label _label
    (:Completed
      (if (or (CallFunction|IsMagazineEmpty) (CallFunction|IsReloading))
        (goto _label Reset)
        (else
          (Utilities|FlowControl|Sequence
            (:then_0
              (Variables|Default|SetIs%20Firing true)
              (Utilities|FlowControl|Sequence
                (:then_0
                  ;[1 0.2263 0.05616] Spawn sound at muzzle
                  (Utilities|IsValid (.sound _fire_sound)
                    (:Is%20Valid
                      (Audio|PlaySoundatLocation (.sound _fire_sound) (.location _returnvalue_2) (.rotation _returnvalue_2) (.volumemultiplier _fire_sound) (.pitchmultiplier _fire_sound) 0.0 (.attenuationsettings _fire_sound) 0 (Components|GetOwner)))))
                (:then_1
                  ;[0.6152 1 0.3901] Spawn particle emitter
                  (Utilities|IsValid _fire_particle_system
                    (:Is%20Valid
                      (Effects|SpawnEmitterAttached _fire_particle_system _mesh _returnvalue "0, 0, 0" "0, 0, 0" "1.000000,1.000000,1.000000" "SnapToTarget"))))
                (:then_2
                  ;[0.4214 1 0] Accumulate recoil
                  (|SetBy-RefVar _recoil (CallFunction|Saturate (+ _recoil (CallFunction|GetRecoilRate) (Utilities|Time|GetWorldDeltaSeconds)))))
                (:then_3
                  (CallFunction|AddMagazine (* (Variables|Stats|Ammo|GetAmmo%20Cost) -1)))))
            (:then_1
              ;[0.8665 0.2257 1] Fire mode handling
              (Utilities|FlowControl|Delay (CallFunction|GetFireDelay))
              (Variables|Default|SetIs%20Firing false)
              (switch Utilities|FlowControl|Switch|SwitchonEFireMode (Variables|Stats|GetFire%20Mode)
                (:NewEnumerator0
                  (Utilities|FlowControl|DoOnce true) ; enters at Reset
                )
                (:NewEnumerator1
                  (Utilities|FlowControl|DoOnce true) ; enters at Reset
                )
                (:NewEnumerator2
                  (goto _label Reset))))))))))

(event Custom|ReleaseFire
  (bind _returnvalue (Utilities|Name|MakeLiteralName "Muzzle"))
  (bind _fire_particle_system (Variables|Effects|GetFire%20Particle%20System))
  (bind _recoil (Variables|Stats|Recoil|GetRecoil))
  (bind _mesh (Variables|Default|GetMesh))
  (bind _fire_sound (Variables|Effects|GetFire%20Sound))
  (bind _returnvalue_2 (Transformation|GetSocketTransform _mesh _returnvalue "RTS_World"))
  ;[0.8665 0.2257 1] Fire mode handling
  (Utilities|FlowControl|DoOnce true
    (:Completed
      (switch Utilities|FlowControl|Switch|SwitchonEFireMode (Variables|Stats|GetFire%20Mode)
        (:NewEnumerator0
          (Utilities|FlowControl|DoOnce false) ; enters at Reset
        )
        (:NewEnumerator1
          (Utilities|FlowControl|DoOnce false) ; enters at Reset
        )))))

(event EventTick
  (params (DeltaSeconds :type Float%20%28single-precision%29))
  (bind _recoil (Variables|Stats|Recoil|GetRecoil))
  ;[0.6671 1 0.3541] Recoil cooldown
  (|SetBy-RefVar _recoil (Math|Interpolation|FInterpTo _recoil 0.0 (Utilities|Time|GetWorldDeltaSeconds) (* (Variables|Stats|Recoil|GetCooldown%20Rate) (Math|Float|SelectFloat 1.0 (Variables|Stats|Recoil|GetIdle%20Cooldown%20Multiplier) (Variables|Default|GetIs%20Firing))))))

(event EventBeginPlay
  ;[1 0.1036 0] Init
  (Variables|Stats|Recoil|SetRecoil 0.0)
  (Variables|Default|SetIs%20Firing false))

(fn GetFireDelay
  (return (/ 1.0 (/ (Variables|Stats|GetRounds%20Per%20Minute) 6e+01))))

(fn IsAiming
  (return (>= (Variables|Default|GetAim) 0.05)))

(fn GetRecoilRate
  (bind _recoil_rate (Variables|Stats|Recoil|GetRecoil%20Rate))
  (return (Math|Float|Lerp _recoil_rate (* _recoil_rate (Variables|Stats|Recoil|GetAiming%20Recoil%20Multiplier)) (Variables|Default|GetAim))))

(fn Initialize
  (params (Mesh :type Primitive%20Component%20Object%20Reference))
  (Variables|Default|SetMesh Mesh))