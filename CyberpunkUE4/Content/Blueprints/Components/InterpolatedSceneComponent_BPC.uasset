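; Scene component that smoothly follows its attach parent, with position, rotation and scale each optionally interpolated.
; On BeginPlay it makes interpolated channels absolute and caches the starting relative transform as an offset.
; Each Tick eases those channels toward the parent transform composed with that offset.
; Each channel has its own speed and can modulate it by a smoothed owner velocity magnitude, normalized against a maximum.
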(event EventTick
  (params (DeltaSeconds :type Float%20%28single-precision%29))
  (bind _returnvalue (Utilities|Time|GetWorldDeltaSeconds))
  (bind _returnvalue_2 (Transformation|GetAttachParent))
  (bind _returnvalue_3 (Transformation|GetWorldTransform))
  (bind _relative_offset (Variables|Interpolation|GetRelative%20Offset))
  (bind _returnvalue_4 (Transformation|GetWorldTransform _returnvalue_2))
  (bind _returnvalue_5 (Math|Transform|ComposeTransforms _relative_offset _returnvalue_4))
  (Utilities|FlowControl|Sequence
    (:then_0
      (if (Math|Boolean|ORBoolean (.scalebyownervelocity (Variables|Interpolation|GetInterpolate%20Position)) (.scalebyownervelocity (Variables|Interpolation|GetInterpolate%20Rotation)) (.scalebyownervelocity (Variables|Interpolation|GetInterpolate%20Scale)))
        (Variables|Interpolation|SetOwner%20Velocity (Math|Interpolation|FInterpTo (Variables|Interpolation|GetOwner%20Velocity) (Math|Vector|VectorLength (Transformation|GetVelocity (Components|GetOwner))) (Utilities|Time|GetWorldDeltaSeconds) (Variables|Interpolation|GetOwner%20Velocity%20Interpolation%20Speed))) ; cache velocity
      ))
    (:then_1
      (Utilities|FlowControl|Sequence
        (:then_0
          (bind (_delta_scale _sweep _teleport) (Utilities|OnInterpolate (Variables|Interpolation|GetInterpolate%20Position))
            (:true
              (Transformation|SetWorldLocation (Math|Interpolation|VInterpTo (.location _returnvalue_3) (.location _returnvalue_5) _returnvalue _delta_scale) _sweep _teleport))))
        (:then_1
          (bind (_delta_scale_2 _sweep_2 _teleport_2) (Utilities|OnInterpolate (Variables|Interpolation|GetInterpolate%20Rotation))
            (:true
              (Transformation|SetWorldRotation (Math|Interpolation|RInterpTo (.rotation _returnvalue_3) (.rotation _returnvalue_5) _returnvalue _delta_scale_2) _sweep_2 _teleport_2))))
        (:then_2
          (bind _delta_scale_3 (Utilities|OnInterpolate (Variables|Interpolation|GetInterpolate%20Scale))
            (:true
              (Transformation|SetWorldScale3D (Math|Interpolation|VInterpTo (.scale _returnvalue_3) (.scale _returnvalue_5) _returnvalue _delta_scale_3)))))))))

(event EventBeginPlay
  ;[1 1 1] Init transform
  (Transformation|SetAbsolute (.interpolate (Variables|Interpolation|GetInterpolate%20Position)) (.interpolate (Variables|Interpolation|GetInterpolate%20Rotation)) (.interpolate (Variables|Interpolation|GetInterpolate%20Scale)))
  (Variables|Interpolation|SetRelative%20Offset (Transformation|GetRelativeTransform)))