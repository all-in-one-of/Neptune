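; Rhythm combo controller that prompts beats on a BPM-driven looping timer and checks gamepad face-button presses against them.
; Each tick queues a random starting beat or next beats from BeatRules, matched only on the combo's latest position, resetting when none remain.
; Queued presses extend the combo, and other face-button presses reset it.
; Feedback is debug prints only, and an audio spectrum snippet is left unconnected.
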(event Custom|ResetCombo
  (Utilities|Array|Clear (Variables|Beats|GetCurrent%20Combo)))

(event Custom|AddBeatToCombo
  (params (Beat :type EBeat%20Enum%20%28by%20ref%29 :default "NewEnumerator0"))
  (Utilities|Array|Add (Variables|Beats|GetCurrent%20Combo) Beat))

(event Custom|BeatLoop
  (bind _beat_queue (Variables|Beats|GetBeat%20Queue))
  (CallFunction|+= (Variables|Default|GetElapsed%20Time) (CallFunction|GetBeatStep))
  (Utilities|FlowControl|Sequence
    (:then_0
      (if (CallFunction|IsBeatComboEmpty)
        (bind (_beat _selected_beat) (CallFunction|GetInitialBeat))
        (|SetBy-RefVar _beat_queue (Utilities|Array|MakeArray _beat))
        (if _selected_beat
          (Development|PrintString (Utilities|String|Append "Initial Beat: " (Utilities|String|EnumtoString _beat)) true true "(R=1.000000,G=0.042460,B=0.273702,A=1.000000)" 4.0))
        (else
          (bind _beats (CallFunction|GetNextBeatsinCombo))
          (if (> (Utilities|Array|Length _beats) 0)
            (|SetBy-RefVar _beat_queue _beats)
            (bind _beat_queue_2 (CallFunction|GetBeatListasString _beats))
            (Development|PrintString (Utilities|String|Append "Next Possible Combos: " _beat_queue_2) true true "(R=0.036277,G=1.000000,B=0.029683,A=1.000000)")
            (else
              (bind _beat_queue_3 (CallFunction|GetBeatListasString (Variables|Beats|GetCurrent%20Combo)))
              (CallFunction|ResetCombo)
              (Development|PrintString (Utilities|String|Append "Final Combo: " _beat_queue_3) true true "(R=1.000000,G=0.432458,B=0.053401,A=1.000000)"))))))))

(event EventBeginPlay
  (Utilities|Time|SetTimerbyEvent (delegate Custom|BeatLoop) (CallFunction|GetBeatStep) true))

(event Input|KeyboardEvents|AnyKey
  (params (Key :type Key%20Structure))
  (:Pressed
    (bind (_beat _valid) (CallFunction|MapKeytoBeat Key))
    (if _valid ; Is valid beat
      (if (Utilities|Array|ContainsItem (Variables|Beats|GetBeat%20Queue) _beat) ; If we hit a beat in a possible combo
        (CallFunction|AddBeattoCombo _beat)
        (bind _beat_queue (CallFunction|GetBeatListasString (Variables|Beats|GetCurrent%20Combo)))
        (Development|PrintString (Utilities|String|Append "Hit beat, current combo: " _beat_queue) true true "(R=0.000000,G=1.000000,B=0.900323,A=1.000000)")
        (else
          (CallFunction|ResetCombo)
          (Development|PrintString "Wrong beat - reset combo" true true "(R=1.000000,G=0.000000,B=0.438449,A=1.000000)"))))))

(fn ConstructionScript)

(fn GetBeatStep
  (return (CallFunction|Integer/Integer(Float) 60 (Variables|Beats|GetBeats%20Per%20Minute))))

(fn GetInitialBeat
  (if (Math|Random|RandomBoolwithWeight (Variables|Beats|GetInitial%20Beat%20Chance))
    (return (Utilities|Enum|ByteToEnumEBeat (Math|Conversions|ToByte(Integer) (Math|Random|RandomIntegerinRange 0 3))) true)
    (else
      (return "NewEnumerator0" false))))

(fn GetNextBeatsinCombo
  (bind _current_combo (Variables|Beats|GetCurrent%20Combo))
  (bind _returnvalue (Utilities|Array|Length _current_combo))
  (bind _returnvalue_2 (Utilities|Array|LastIndex _current_combo))
  (for _array_element (Variables|Beats|GetBeat%20Rules)
    (if (and (> (Utilities|Array|Length (.sequence _array_element)) _returnvalue) (Utilities|Enum|Equal(Enum) (Utilities|Array|Get(acopy) _current_combo _returnvalue_2) (Utilities|Array|Get(acopy) (.sequence _array_element) _returnvalue_2)))
      (Utilities|Array|Add (LocalVariables|GetNext%20Beats) (Utilities|Array|Get(acopy) (.sequence _array_element) _returnvalue))))
  (return (LocalVariables|GetNext%20Beats)))

(fn IsBeatComboEmpty
  (return (<= (Utilities|Array|Length (Variables|Beats|GetCurrent%20Combo)) 0)))

(fn GetBeatListasString
  (params (Beat%20List :type Array%20of%20EBeat%20Enums :default "NewEnumerator0"))
  (bind _result (LocalVariables|GetResult))
  (for _array_element Beat%20List
    (|SetBy-RefVar _result (Utilities|String|Append _result (Utilities|String|EnumtoString _array_element))))
  (return (LocalVariables|GetResult)))

(fn MapKeytoBeat
  (params (Key :type Key%20Structure))
  (if (== Key "Gamepad_FaceButton_Bottom")
    (return "NewEnumerator0" true)
    (elif (== Key "Gamepad_FaceButton_Right")
      (return "NewEnumerator1" true)
      (elif (== Key "Gamepad_FaceButton_Left")
        (return "NewEnumerator2" true)
        (elif (== Key "Gamepad_FaceButton_Top")
          (return "NewEnumerator3" true)
          (else
            (return "NewEnumerator0" false) ; invalid key
          ))))))