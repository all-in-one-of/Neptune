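; Base static mesh actor Blueprint in Tools with helper functions for placing, rotating and mirroring itself, apparently for level dressing.
; The construction script optionally sets a random yaw within plus or minus YawRange, resetting pitch and roll to zero.
; MoveToFloor snaps to a downward visibility trace hit, while Rotate and Flip functions add world rotation steps or invert relative scale per axis.
; BeginPlay destroys the Billboard component.
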(event EventBeginPlay
  (Components|DestroyComponent (Variables|Default|GetBillboard)))

(event Collision|EventActorBeginOverlap
  (params (OtherActor :type Actor%20Object%20Reference)))

(event EventTick
  (params (DeltaSeconds :type Float%20%28single-precision%29)))

(fn ConstructionScript
  (bind _yaw_range (Variables|StaticMesh|Randomisation|GetYaw%20Range))
  (if (Variables|StaticMesh|Randomisation|GetAdd%20Random%20Yaw)
    (Transformation|SetActorRelativeRotation (Math|Rotator|MakeRotator 0.0 0.0 (Math|Random|RandomFloatinRange (* _yaw_range -1.0) _yaw_range)))))

(fn MovetoFloor
  (bind _returnvalue (Transformation|GetActorLocation))
  (bind (_outhit _returnvalue_2) (Collision|LineTraceByChannel _returnvalue (+ _returnvalue "0, 0,-5000.000000") "TraceTypeQuery1" true 0 "None"))
  (if _returnvalue_2
    (Transformation|SetActorLocation (.location _outhit) false false)))

(fn RotateX
  (Class|Actor|AddActorWorldRotation (Math|Rotator|MakeRotator (Variables|StaticMesh|GetRotation%20Increment) 0.0 0.0)))

(fn RotateY
  (Class|Actor|AddActorWorldRotation (Math|Rotator|MakeRotator 0.0 (Variables|StaticMesh|GetRotation%20Increment) 0.0)))

(fn RotateZ
  (Class|Actor|AddActorWorldRotation (Math|Rotator|MakeRotator 0.0 0.0 (Variables|StaticMesh|GetRotation%20Increment))))

(fn FlipX
  (bind _returnvalue (Class|Actor|GetActorRelativeScale3D))
  (Transformation|SetActorRelativeScale3D (Math|Vector|MakeVector (CallFunction|Invert (.x _returnvalue)) (.y _returnvalue) (.z _returnvalue))))

(fn FlipY
  (bind _returnvalue (Class|Actor|GetActorRelativeScale3D))
  (Transformation|SetActorRelativeScale3D (Math|Vector|MakeVector (.x _returnvalue) (CallFunction|Invert (.y _returnvalue)) (.z _returnvalue))))

(fn FlipZ
  (bind _returnvalue (Class|Actor|GetActorRelativeScale3D))
  (Transformation|SetActorRelativeScale3D (Math|Vector|MakeVector (.x _returnvalue) (.y _returnvalue) (CallFunction|Invert (.z _returnvalue)))))