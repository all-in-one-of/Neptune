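; Spline tool actor that lays a chosen static mesh along a spline as deformed spline mesh segments, extending a parent spline Blueprint.
; Construct optionally resamples the spline by inserting points at intervals, then builds one segment per point pair using tangents, scale and roll.
; AddSplineMesh applies collision, shadow and physical material settings, with material overrides set per segment.
; RefreshSpline destroys old segments before deferring to the parent; the construction script adds up/right arrows at each point.
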(event EventBeginPlay
  (|CallParentFunction))

(event Collision|EventActorBeginOverlap
  (params (OtherActor :type Actor%20Object%20Reference)))

(event EventTick
  (params (DeltaSeconds :type Float%20%28single-precision%29)))

(fn ConstructionScript
  (bind _spline (Variables|Default|GetSpline))
  (bind _spline_2 (Variables|Default|GetSpline))
  (|CallParentFunction)
  (for _index (range 0 (- (Spline|GetNumberOfSplinePoints (Variables|Default|GetSpline)) 1))
    (Utilities|FlowControl|Sequence
      (:then_0
        (bind _returnvalue (AddComponent|AddArrowComponent false))
        (Transformation|SetWorldLocationAndRotation _returnvalue (Spline|GetLocationatSplinePoint _spline _index "World") (Math|Conversions|RotationFromXVector (Class|SplineComponent|GetUpVectoratSplinePoint _spline _index "World")) false false))
      (:then_1
        (bind _returnvalue_2 (AddComponent|AddArrowComponent false))
        (Transformation|SetWorldLocationAndRotation _returnvalue_2 (Spline|GetLocationatSplinePoint _spline_2 _index "World") (Math|Conversions|RotationFromXVector (Class|SplineComponent|GetRightVectoratSplinePoint _spline_2 _index "Local")) false false)))))

(fn Construct
  (bind _spline (Variables|Default|GetSpline))
  (bind _global_scale (Variables|SplineMesh|GetGlobal%20Scale))
  (|CallParentFunction)
  (Spline|Resample|ResampleSpline)
  (Utilities|FlowControl|Sequence
    (:then_0
      (for _index (range (Class|KismetSystemLibrary|MakeLiteralInteger) (- (Spline|GetNumberOfSplinePoints (Variables|Default|GetSpline)) 2))
        (bind _returnvalue (SplineMesh|AddSplineMesh))
        (Utilities|FlowControl|Sequence
          (:then_0
            (Components|StaticMesh|SetStaticMesh _returnvalue (Variables|SplineMesh|Assets|GetSpline%20Mesh))
            (SplineMesh|SetForwardAxis _returnvalue (Variables|SplineMesh|GetForward%20Axis) false)
            (SplineMesh|SetSplineUpDir _returnvalue (Math|Vector|Normalize (Variables|SplineMesh|GetUp%20Vector)) false)
            ;[1 0.1335 0.2734] Override materials if there any
            (for (_array_element _array_index) (Variables|SplineMesh|Assets|GetMaterial%20Overrides)
              (Rendering|Material|SetMaterial _returnvalue _array_index _array_element)))
          (:then_1
            (SplineMesh|SetStartandEnd _returnvalue (.Location (Spline|GetLocationandTangentatSplinePoint _spline _index "Local")) (.Tangent (Spline|GetLocationandTangentatSplinePoint _spline _index "Local")) (.Location (Spline|GetLocationandTangentatSplinePoint _spline (+ _index 1) "Local")) (.Tangent (Spline|GetLocationandTangentatSplinePoint _spline (+ _index 1) "Local")) false :!class /Script/Engine.SplineMeshComponent))
          (:then_2
            (SplineMesh|SetStartScale _returnvalue (* (Math|Vector2D|MakeVector2D (.y (Spline|GetScaleatSplinePoint _spline _index)) (.z (Spline|GetScaleatSplinePoint _spline _index))) _global_scale) false :!class /Script/Engine.SplineMeshComponent)
            (Class|SplineMeshComponent|SetStartRoll _returnvalue (/ (.roll (Spline|GetRotationatSplinePoint _spline _index "Local")) 3.6e+02) false)
            (Class|SplineMeshComponent|SetEndRoll _returnvalue (/ (.roll (Spline|GetRotationatSplinePoint _spline (+ _index 1) "Local")) 3.6e+02) false))
          (:then_3
            (SplineMesh|SetEndScale _returnvalue (* _global_scale (Math|Vector2D|MakeVector2D (.y (Spline|GetScaleatSplinePoint _spline (+ _index 1))) (.z (Spline|GetScaleatSplinePoint _spline (+ _index 1))))) true :!class /Script/Engine.SplineMeshComponent)))))
    (:then_1
      (return true))))

(fn RefreshSpline
  (params (Construct :type Boolean))
  (Utilities|FlowControl|Sequence
    (:then_0
      (for _array_element (Actor|GetComponentsByClass "/Script/Engine.SplineMeshComponent")
        (Components|DestroyComponent _array_element)))
    (:then_1
      (bind _successful (|CallParentFunction true))
      (return _successful))))

(fn AddSplineMesh
  (bind _physics_material_override (Variables|SplineMesh|Collision|GetPhysics%20Material%20Override))
  (bind _returnvalue (AddComponent|AddSplineMeshComponent false))
  (Utilities|FlowControl|Sequence
    (:then_0
      ;[0.2188 0.5199 1] Collision
      (CallFunction|SetPrimitiveCollision _returnvalue (Variables|SplineMesh|Collision|GetCollision%20Enabled) (Variables|SplineMesh|Collision|GetCollision%20Channel) "ECR_Block" (Variables|SplineMesh|Collision|GetCollision%20Responses) (Variables|SplineMesh|Collision|GetCan%20Character%20Step%20Up%20On))
      (Rendering|SetCastShadow _returnvalue (Variables|SplineMesh|Assets|GetCast%20Shadow)))
    (:then_1
      ;[1 0.5125 0.0772] Physics material override
      (if (!= _physics_material_override 0)
        (Class|PrimitiveComponent|SetPhysMaterialOverride _returnvalue _physics_material_override)))
    (:then_2
      (return _returnvalue))))

(fn ResampleSpline
  (bind _accumulated_dist (LocalVariables|GetAccumulated%20Dist))
  (bind _spline (Variables|Default|GetSpline))
  (if (Variables|Spline|Resample|GetResample%20Spline?)
    (while (< (LocalVariables|GetAccumulated%20Dist) (Spline|GetSplineLength (Variables|Default|GetSpline)))
      (Utilities|FlowControl|Sequence
        (:then_0
          (Spline|AddSplinePointatIndex _spline (Spline|GetLocationatDistanceAlongSpline _spline _accumulated_dist "Local") (CallFunction|GetNearestPointatDistance _accumulated_dist) "Local" true))
        (:then_1
          (CallFunction|+= (LocalVariables|GetAccumulated%20Dist) (Variables|Default|GetResample%20Width)))))))