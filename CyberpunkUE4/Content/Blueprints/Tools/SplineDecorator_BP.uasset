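; Spline decorator tool that scatters static mesh components, picked at random from DecoratorAssets, along a spline.
; Construct steps by Density times spline Z scale, composing each asset's randomised transform, combined with GlobalTransform, onto the spline transform, with Y scale applied uniformly.
; Meshes receive configurable mobility, collision and physics.
; Randomness draws from a stream, and RandomiseSeed picks a new seed, destroys the meshes and calls Construct again.
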(event EventBeginPlay
  (|CallParentFunction) ; This node is disabled and will not be called.\nDrag off pins to build functionality.
)

(event Collision|EventActorBeginOverlap
  (params (OtherActor :type Actor%20Object%20Reference)))

(event EventTick
  (params (DeltaSeconds :type Float%20%28single-precision%29)))

(fn ConstructionScript
  (|CallParentFunction))

(fn Construct
  (bind _spline (Variables|Default|GetSpline))
  (bind _stream (Variables|SplineDecorator|GetStream))
  (bind _accum_distance (LocalVariables|GetAccum%20Distance))
  (bind _accum_distance_2 (LocalVariables|GetAccum%20Distance))
  (bind _decorator_assets (Variables|SplineDecorator|GetDecorator%20Assets))
  (bind _returnvalue (Utilities|Array|LastIndex _decorator_assets))
  (bind _returnvalue_2 (Spline|GetTransformatDistanceAlongSpline _spline _accum_distance "Local" true))
  (bind _returnvalue_3 (Math|Random|RandomIntegerinRangefromStream 0 _returnvalue _stream))
  (bind _output (Utilities|Array|Get(acopy) _decorator_assets _returnvalue_3))
  (|CallParentFunction)
  (Utilities|FlowControl|Sequence
    (:then_0
      (while (<= (LocalVariables|GetAccum%20Distance) (Spline|GetSplineLength (Variables|Default|GetSpline)))
        (Utilities|FlowControl|Sequence
          (:then_0
            (bind _returnvalue_4 (CallFunction|AddStaticMeshComponent false (Math|Transform|ComposeTransforms (SplineDecorator|GetRandomTransform (SplineDecorator|CombineFTransforms (.transform _output) (Variables|SplineDecorator|GetGlobal%20Transform))) (Math|Transform|MakeTransform (.location _returnvalue_2) (Utilities|Select :Index (.splinespace _output) :Option%200 (.rotation _returnvalue_2) :Option%201 (.rotation (Spline|GetTransformatDistanceAlongSpline _spline _accum_distance "World" true))) (Math|Vector|MakeVector (.y (.scale _returnvalue_2)) (.y (.scale _returnvalue_2)) (.y (.scale _returnvalue_2))))) (Variables|SplineDecorator|GetMoveable)))
            (Components|StaticMesh|SetStaticMesh _returnvalue_4 (.staticmesh _output))
            (Physics|SetSimulatePhysics _returnvalue_4 (Variables|SplineDecorator|GetSimulate%20Phyiscs))
            (Utilities|Array|Add (Variables|SplineDecorator|GetSpline%20Meshes) _returnvalue_4))
          (:then_1
            (CallFunction|+= _accum_distance_2 (* (Variables|SplineDecorator|GetDensity) (.z (Class|SplineComponent|GetScaleatDistanceAlongSpline (Variables|Default|GetSpline) _accum_distance_2))))))))
    (:then_1
      (return true))))

(fn RandomiseSeed
  (Variables|SplineDecorator|SetSeed (Math|Random|RandomIntegerinRange 0 100000))
  (for _array_element (Variables|SplineDecorator|GetSpline%20Meshes)
    (Components|DestroyComponent _array_element))
  (CallFunction|Construct))

(fn GetRandomTransform
  (params (In :type F%20Randomised%20Transform%20Structure))
  (bind (_roll _pitch _yaw) (Math|Rotator|BreakRotator (.randomrotation In)))
  (bind _output (SplineDecorator|GetRandomVector (.randomlocation In)))
  (bind _returnvalue (Math|Transform|MakeTransform (.location In) (.rotation In)))
  (bind (_x _y) (Math|Vector2D|BreakVector2D (.randomuniformscalerange In)))
  (bind _stream (Variables|SplineDecorator|GetStream))
  (bind _returnvalue_2 (Math|Random|RandomFloatinRangefromStream _x _y _stream))
  (bind _output_2 (SplineDecorator|GetRandomVector (Math|Vector|MakeVector _roll _pitch _yaw)))
  (bind _returnvalue_3 (Math|Rotator|MakeRotator (.x _output_2) (.y _output_2) (.z _output_2)))
  (bind _returnvalue_4 (Math|Transform|MakeTransform _output _returnvalue_3 (Math|Vector|MakeVector _returnvalue_2 _returnvalue_2 _returnvalue_2)))
  (bind (_location _rotation _scale) (Math|Transform|BreakTransform _returnvalue_4))
  (return (Math|Transform|ComposeTransforms (Math|Transform|MakeTransform _location (Utilities|Select :Index (.randomtransformspace In) :Option%200 _rotation :Option%201 (.rotation (Math|Transform|ComposeTransforms _returnvalue_4 (Transformation|GetActorTransform)))) _scale) (Math|Transform|MakeTransform (.location _returnvalue) (.rotation _returnvalue) (* (.scale _returnvalue) (* (.scale In) (.uniformscale In)))))))

(fn GetRandomVector
  (params (Input :type Vector))
  (bind _returnvalue (* Input -1.0))
  (bind (_x _y _z) (Math|Vector|BreakVector Input))
  (bind _stream (Variables|SplineDecorator|GetStream))
  (return (Math|Vector|MakeVector (Math|Random|RandomFloatinRangefromStream (.x _returnvalue) _x _stream) (Math|Random|RandomFloatinRangefromStream (.y _returnvalue) _y _stream) (Math|Random|RandomFloatinRangefromStream (.z _returnvalue) _z _stream))))

(fn CombineFTransforms
  (params (A :type F%20Randomised%20Transform%20Structure) (B :type F%20Randomised%20Transform%20Structure))
  (return (Utilities|Struct|MakeFRandomisedTransform "NewEnumerator1" (+ (.location A) (.location B)) (Math|Rotator|CombineRotators (.rotation A) (.rotation B)) (* (.scale A) (.scale B)) (* (.uniformscale A) (.uniformscale B)) "NewEnumerator1" (+ (.randomlocation A) (.randomlocation B)) (Math|Rotator|CombineRotators (.randomrotation A) (.randomrotation B)) (* (.randomuniformscalerange A) (.randomuniformscalerange B)))))

(fn AddStaticMeshComponent
  (params (bManualAttachment :type Boolean) (RelativeTransform :type Transform) (Moveable :type Boolean))
  (Utilities|FlowControl|Sequence
    (:then_0
      (if Moveable
        (AddComponent|AddStaticMeshComponent bManualAttachment RelativeTransform)
        (else
          (AddComponent|AddStaticMeshComponent bManualAttachment RelativeTransform))))
    (:then_1
      (CallFunction|SetPrimitiveCollision (LocalVariables|GetStatic%20Mesh) (Variables|SplineDecorator|Collision|GetCollision%20Enabled) (select (Variables|SplineDecorator|GetSimulate%20Phyiscs) "ECC_PhysicsBody" (Variables|SplineDecorator|Collision|GetCollision%20Channel)) "ECR_Block" (Variables|SplineDecorator|Collision|GetCollision%20Responses) (Variables|SplineDecorator|Collision|GetCan%20Character%20Step%20Up%20On)))
    (:then_2
      (return (LocalVariables|GetStatic%20Mesh)))))