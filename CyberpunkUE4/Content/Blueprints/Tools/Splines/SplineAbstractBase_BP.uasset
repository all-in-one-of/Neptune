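; Abstract base actor for spline tools that build content from modifier and generator components.
; Construction updates splines, then modifiers, then generators, in that order so reparam tables and generated splines exist first.
; It also draws optional instanced gizmos at spline points, optionally including modifier-generated splines, and clears them on BeginPlay.
; Helper functions create spline and mesh components, clear owned components and randomise generator seeds.
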(event EventBeginPlay
  (|CallParentFunction)
  (Utilities|FlowControl|Sequence
    (:then_0
      (Gizmos|ClearGizmos))
    (:then_1
      (CallFunction|SetActorTickSettings self (Variables|ActorTick|GetTick%20Settings)))))

(fn ConstructionScript
  (|CallParentFunction)
  (SplineBase|Construct))

(fn Construct
  (Components|GenerateandUpdateComponents)
  (Gizmos|GenerateGizmos)
  (return true))

(fn GenerateandUpdateComponents
  (Utilities|FlowControl|Sequence
    (:then_0
      ;[1 0.03936 0] Order is important
      ; Must update spline reparam table first
      ; Then update spline modifiers to generate the spline components needed by the generators
      (bind _spline_components (Components|Getters|GetAllSplineComponents))
      (Spline|UpdateSpline _spline_components))
    (:then_1
      (bind _spline_modifiers (Components|Getters|GetAllSplineModifierComponents))
      (Default|UpdateComponent _spline_modifiers))
    (:then_2
      (bind _spline_generators (Components|Getters|GetAllSplineGeneratorComponents))
      (Default|UpdateComponent _spline_generators))))

(fn AddSplineMeshComponent
  (params (Mobility :type EComponentMobility%20Enum :default "Static") (Relative%20Transform :type Transform) (Visibility :type Boolean) (Hidden%20In%20Game :type Boolean))
  (bind _returnvalue (AddComponent|AddSplineMeshComponent false Relative%20Transform))
  (Transformation|SetMobility _returnvalue Mobility)
  (Rendering|SetVisibility _returnvalue Visibility false)
  (Development|SetHiddeninGame _returnvalue Hidden%20In%20Game false)
  (return _returnvalue))

(fn ClearComponents
  (bind _spline_base_components (Components|Getters|GetAllSplineBaseComponents))
  (Default|ClearOwnedComponents _spline_base_components))

(fn DestroyComponent
  (params (Component :type Actor%20Component%20Object%20Reference))
  (Components|DestroyComponent Component))

(fn GenerateGizmos
  (bind _gizmo_scale (Variables|Gizmos|GetGizmo%20Scale))
  (Utilities|FlowControl|Sequence
    (:then_0
      (Gizmos|ClearGizmos))
    (:then_1
      (if (Variables|Gizmos|GetDraw%20Gizmos)
        (bind _splines (Components|Getters|GetAllModifierSplines))
        (bind _spline_component (Utilities|ForEachSplineComponent self)
          (:LoopBody
            (if (or (== (Utilities|Array|FindItem _splines _spline_component) -1) (Variables|Gizmos|GetDraw%20Gizmos%20On%20Modifier%20Splines))
              (bind (_spline _index) (Utilities|ForEachSplinePoint _spline_component 0 0 false)
                (:LoopBody
                  (Components|InstancedStaticMesh|AddInstance (Variables|Default|GetGizmos) (Math|Transform|ComposeTransforms (Math|Transform|MakeTransform (Spline|GetLocationatSplinePoint _spline _index "Local") (Spline|GetRotationatSplinePoint _spline _index "Local") (Math|Vector|MakeVector _gizmo_scale _gizmo_scale _gizmo_scale)) (Transformation|GetRelativeTransform _spline))))))))))))

(fn GetAllSplineComponents
  (return (Actor|GetComponentsByClass "/Script/Engine.SplineComponent")))

(fn GetAllSplineBaseComponents
  (return (Actor|GetComponentsByClass "/Game/Blueprints/Tools/Splines/Components/BaseComponents/SplineComponentBase_BPC.SplineComponentBase_BPC_C")))

(fn ClearGizmos
  (Components|InstancedStaticMesh|ClearInstances (Variables|Default|GetGizmos)))

(fn AddSplineComponent
  (params (Mobility :type EComponentMobility%20Enum :default "Static") (RelativeTransform :type Transform))
  (bind _returnvalue (AddComponent|AddSplineComponent false RelativeTransform))
  (Transformation|SetMobility _returnvalue Mobility)
  (return _returnvalue))

(fn GetAllSplineModifierComponents
  (return (Actor|GetComponentsByClass "/Game/Blueprints/Tools/Splines/Components/SplineModifier_BPC.SplineModifier_BPC_C")))

(fn GetAllSplineGeneratorComponents
  (return (Actor|GetComponentsByClass "/Game/Blueprints/Tools/Splines/Components/BaseComponents/SplineGeneratorBase_BPC.SplineGeneratorBase_BPC_C")))

(fn GetAllModifierSplines
  (bind _spline_modifiers (Components|Getters|GetAllSplineModifierComponents))
  (for _array_element _spline_modifiers
    (Utilities|Array|Add (LocalVariables|GetModifier%20Splines) (Variables|/Game/Blueprints/Tools/Splines/Components/SplineModifier_BPC.SplineModifier_BPC_C|GetGenerated%20Spline _array_element)))
  (return (LocalVariables|GetModifier%20Splines)))

(fn AddHierarchialInstancedStaticMeshComponent
  (params (Mobility :type EComponentMobility%20Enum :default "Static") (RelativeTransform :type Transform))
  (bind _returnvalue (AddComponent|AddHierarchicalInstancedStaticMeshComponent false RelativeTransform))
  (Transformation|SetMobility _returnvalue Mobility)
  (return _returnvalue))

(fn AddStaticMeshComponent
  (params (Mobility :type EComponentMobility%20Enum :default "Static") (RelativeTransform :type Transform))
  (bind _returnvalue (AddComponent|AddStaticMeshComponent false RelativeTransform))
  (Transformation|SetMobility _returnvalue Mobility)
  (return _returnvalue))

(fn RandomiseSeed
  (bind _spline_generators (Components|Getters|GetAllSplineGeneratorComponents))
  (Default|RandomiseSeed _spline_generators))