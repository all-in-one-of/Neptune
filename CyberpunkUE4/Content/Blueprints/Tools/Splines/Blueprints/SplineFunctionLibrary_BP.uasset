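; Blueprint function library of shared helpers for spline tools, covering transform math, spline editing, tick settings and procedural mesh cleanup.
; Spline helpers sample location, tangent, normal, roll and scale by point or distance, copy points between splines, and force point types.
; GetRandomTransform builds seeded offsets from a random stream.
; MergeProceduralMeshSections appends sections into section 0, shifting triangles by a running index count, while RemoveUnusedSections clears empty ones.
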(fn UniformScaleTransform
  (params (Transform :type Transform) (Uniform%20Scale :type Float%20%28single-precision%29))
  (return (Math|Transform|MakeTransform (.location Transform) (.rotation Transform) (* (.scale Transform) Uniform%20Scale))))

(fn TransformtoScale2D
  (params (Transform :type Transform))
  (return (Math|Vector2D|MakeVector2D (.y (.scale Transform)) (.z (.scale Transform)))))

(fn CombineRelativeTransforms
  (params (A :type Transform) (B :type Transform))
  (return (Math|Transform|MakeTransform (+ (.location A) (.location B)) (Math|Rotator|CombineRotators (.rotation A) (.rotation B)) (* (.scale A) (.scale B)))))

(fn Scale2DTransform
  (params (Transform :type Transform) (Scale2D :type Vector%202D%20Structure))
  (return (Math|Transform|MakeTransform (.location Transform) (.rotation Transform) (* (.scale Transform) (Math|Vector|MakeVector 1.0 (.x Scale2D) (.y Scale2D))))))

(fn RollTransform
  (params (Transform :type Transform) (Roll :type Float%20%28single-precision%29))
  (return (Math|Transform|MakeTransform (.location Transform) (Math|Rotator|CombineRotators (.rotation Transform) (Math|Rotator|MakeRotator Roll 0.0 0.0)) (.scale Transform))))

(fn TransformtoRoll
  (params (Transform :type Transform))
  (return (.roll (.rotation Transform))))

(fn TransformtoOffset2D
  (params (Transform :type Transform))
  (return (Math|Vector2D|MakeVector2D (.y (.location Transform)) (.z (.location Transform)))))

(fn OffsetPositionfromTangent
  (params (Position :type Vector) (Tangent :type Vector :default "1.000000,0,0") (Scale :type Float%20%28single-precision%29))
  (return (+ Position (* (Math|Vector|Normalize Tangent) Scale))))

(fn GetLocationandTangentatDistanceAlongSpline
  (params (Target :type Spline%20Component%20Object%20Reference) (Distance :type Float%20%28single-precision%29) (CoordinateSpace :type ESplineCoordinateSpace%20Enum :default "Local") (Step%20Width :type Float%20%28single-precision%29))
  (bind _returnvalue (Spline|GetTangentatDistanceAlongSpline Target Distance CoordinateSpace))
  (return (Spline|GetLocationatDistanceAlongSpline Target Distance CoordinateSpace) _returnvalue (* (Math|Vector|Normalize _returnvalue) Step%20Width)))

(fn SetActorTickSettings
  (params (Actor :type Actor%20Object%20Reference) (Tick%20Settings :type F%20Tick%20Settings%20Structure))
  (Actor|Tick|SetActorTickEnabled Actor (.tickenabled Tick%20Settings))
  (Actor|Tick|SetActorTickInterval Actor (.tickinterval Tick%20Settings))
  (Components|Tick|SetTickGroup Actor (.tickgroup Tick%20Settings)))

(fn SetComponentTickSettings
  (params (Component :type Actor%20Component%20Object%20Reference) (Tick%20Settings :type F%20Tick%20Settings%20Structure))
  (Components|Tick|SetComponentTickEnabled Component (.tickenabled Tick%20Settings))
  (Class|ActorComponent|SetComponentTickInterval Component (.tickinterval Tick%20Settings))
  (Components|Tick|SetTickGroup Component (.tickgroup Tick%20Settings)))

(fn GetAxisfromVector
  (params (Vector :type Vector) (Axis :type ESplineMeshAxis%20Enum :default "X"))
  (return (Utilities|Select :Index Axis :X (.x Vector) :Y (.y Vector) :Z (.z Vector))))

(fn DuplicateSplinePoints
  (params (Source%20Spline :type Spline%20Component%20Object%20Reference) (Destination%20Spline :type Spline%20Component%20Object%20Reference))
  (Spline|ClearSplinePoints Destination%20Spline false)
  (bind (_spline _index) (Utilities|ForEachSplinePoint Source%20Spline 0 0 false)
    (:LoopBody
      (Utilities|FlowControl|Sequence
        (:then_0
          (Spline|AddSplinePointatIndex Destination%20Spline (Spline|GetLocationatSplinePoint _spline _index "Local") _index "Local" false))
        (:then_1
          (Spline|SetTangentsatSplinePoint Destination%20Spline _index (Spline|GetArriveTangentatSplinePoint _spline _index "Local") (Spline|GetLeaveTangentatSplinePoint _spline _index "Local") "Local" false))
        (:then_2
          (Class|SplineComponent|SetUpVectoratSplinePoint Destination%20Spline _index (Class|SplineComponent|GetUpVectoratSplinePoint _spline _index "Local") "Local" false))
        (:then_3
          (Class|CyberpunkSplineFunctionLibrary|SetScaleatSplinePoint Destination%20Spline _index (Spline|GetScaleatSplinePoint _spline _index) false))))
    (:Completed
      (Spline|UpdateSpline Destination%20Spline))))

(fn SetSplineColours
  (params (Target :type Spline%20Component%20Object%20Reference) (Unselected%20Colour :type Linear%20Color%20Structure :default "(R=1.000000,G=1.000000,B=1.000000,A=1.000000)") (Selected%20Colour :type Linear%20Color%20Structure :default "(R=1.000000,G=0.000000,B=0.000000,A=1.000000)"))
  (Utilities|FlowControl|Sequence
    (:then_0
      (Class|SplineComponent|SetUnselectedSplineSegmentColor Target Unselected%20Colour))
    (:then_1
      (Class|SplineComponent|SetSelectedSplineSegmentColor Target Selected%20Colour))))

(fn GetNormalatSplinePoint
  (params (Target :type Spline%20Component%20Object%20Reference) (Point%20Index :type Integer) (Coordinate%20Space :type ESplineCoordinateSpace%20Enum :default "Local"))
  (return (Math|Vector|Normalize (Math|Vector|CrossProduct (Class|SplineComponent|GetUpVectoratSplinePoint Target Point%20Index Coordinate%20Space) (Spline|GetTangentatSplinePoint Target Point%20Index Coordinate%20Space)))))

(fn GetNormalatDistanceAlongSpline
  (params (Target :type Spline%20Component%20Object%20Reference) (Distance :type Float%20%28single-precision%29) (Coordinate%20Space :type ESplineCoordinateSpace%20Enum :default "Local"))
  (return (Math|Vector|Normalize (Math|Vector|CrossProduct (Class|SplineComponent|GetUpVectoratDistanceAlongSpline Target Distance Coordinate%20Space) (Spline|GetTangentatDistanceAlongSpline Target Distance Coordinate%20Space)))))

(fn ForceSplinePointType
  (params (Target :type Spline%20Component%20Object%20Reference) (Point%20Type :type ESplinePointType%20Enum :default "Linear"))
  (Utilities|IsValid Target
    (:Is%20Valid
      (bind (_spline _index) (Utilities|ForEachSplinePoint Target 0 0 false)
        (:LoopBody
          (Spline|SetSplinePointType _spline _index Point%20Type false))
        (:Completed
          (Spline|UpdateSpline _spline))))))

(fn GetRandomTransform
  (params (Random%20Transform :type F%20Randomised%20Transform%20Structure) (Stream :type Random%20Stream%20Structure%20%28by%20ref%29))
  (bind ___worldcontext (LocalVariables|Get__WorldContext))
  (bind _out (Transform|Random|GetRandomVectorinStream (.rotation Random%20Transform) Stream ___worldcontext))
  (return (Math|Transform|MakeTransform (Transform|Random|GetRandomVectorinStream (.location Random%20Transform) Stream ___worldcontext) (Math|Rotator|MakeRotator (.x _out) (.y _out) (.z _out)) (* (+ (Transform|Random|GetRandomVectorinStream (.scale Random%20Transform) Stream ___worldcontext) 1.0) (+ (Math|Random|RandomFloatinRangefromStream (CallFunction|Invert (.uniformscale Random%20Transform) ___worldcontext) (.uniformscale Random%20Transform) Stream) 1.0)))))

(fn GetRandomVectorinStream
  (params (In :type Vector) (Stream :type Random%20Stream%20Structure))
  (bind (_x _y _z) (Math|Vector|BreakVector In))
  (bind ___worldcontext (LocalVariables|Get__WorldContext))
  (bind _out (CallFunction|Invert(Vector) In ___worldcontext))
  (return (Math|Vector|MakeVector (Math|Random|RandomFloatinRangefromStream (.x _out) _x Stream) (Math|Random|RandomFloatinRangefromStream (.y _out) _y Stream) (Math|Random|RandomFloatinRangefromStream (.z _out) _z Stream))))

(fn GetTransformandTangentatSplinePoint
  (params (Target :type Spline%20Component%20Object%20Reference) (Index :type Integer) (CoordinateSpace :type ESplineCoordinateSpace%20Enum :default "Local"))
  (bind (_location _tangent) (Spline|GetLocationandTangentatSplinePoint Target Index CoordinateSpace))
  (return _location _tangent (Spline|GetScaleatSplinePoint Target Index) (Spline|GetRollatSplinePoint Target Index CoordinateSpace)))

(fn GetBoundsfromAxis
  (params (Target :type Static%20Mesh%20Object%20Reference) (Axis :type ESplineMeshAxis%20Enum :default "X"))
  (return (Spline|GetAxisfromVector (* (.boxextent (StaticMesh|GetBounds Target)) 2.0) Axis (LocalVariables|Get__WorldContext))))

(fn ForwardAxistoVector
  (params (Forward%20Axis :type ESplineMeshAxis%20Enum :default "X"))
  (return (Utilities|Select :Index Forward%20Axis :X "1.000000, 0, 0" :Y "0,1.000000, 0" :Z "0, 0,1.000000")))

(fn GetTransformandTangentatDistanceAlongSpline
  (params (Target :type Spline%20Component%20Object%20Reference) (Distance :type Float%20%28single-precision%29) (Step%20Width :type Float%20%28single-precision%29) (CoordinateSpace :type ESplineCoordinateSpace%20Enum :default "Local"))
  (bind ___worldcontext (LocalVariables|Get__WorldContext))
  (bind (_location _tangent _corrected_tangent) (Spline|GetLocationandTangentatDistanceAlongSpline Target Distance CoordinateSpace Step%20Width ___worldcontext))
  (return _location _tangent _corrected_tangent (Class|SplineComponent|GetScaleatDistanceAlongSpline Target Distance) (Class|SplineComponent|GetRollatDistanceAlongSpline Target Distance CoordinateSpace)))

(fn MergeProceduralMeshSections
  (params (Procedural%20Mesh%20Component :type Procedural%20Mesh%20Component%20Object%20Reference))
  (bind ___worldcontext (LocalVariables|Get__WorldContext))
  (bind (_procedural_mesh _index) (Utilities|ForEachProceduralMeshSection Procedural%20Mesh%20Component)
    (:LoopBody
      (bind (_vertices _triangles _normals _uvs _tangents) (Class|KismetProceduralMeshLibrary|GetSectionfromProceduralMesh _procedural_mesh _index))
      (bind _output_get (LocalVariables|SetBuffer _triangles))
      (Utilities|FlowControl|Sequence
        (:then_0
          (for (_ _array_index) _output_get
            (|SetBy-RefVar (Utilities|Array|Get(acopy) _output_get _array_index) (+ (Utilities|Array|Get(acopy) _output_get _array_index) (LocalVariables|GetNum%20of%20Indices))))
          (|SetBy-RefVar (LocalVariables|GetNum%20of%20Indices) (+ (LocalVariables|GetNum%20of%20Indices) (Utilities|Array|Length _output_get))))
        (:then_1
          (bind (_vertices_2 _triangles_2 _normals_2 _uvs_2 _tangents_2) (Class|KismetProceduralMeshLibrary|GetSectionfromProceduralMesh _procedural_mesh))
          (Class|ProceduralMeshComponent|CreateMeshSectionLinearColor _procedural_mesh 0 (ProceduralMesh|AppendVectorArray _vertices_2 _vertices ___worldcontext) (ProceduralMesh|AppendIntegerArray _triangles_2 (LocalVariables|GetBuffer) ___worldcontext) (ProceduralMesh|AppendVectorArray _normals_2 _normals ___worldcontext) (ProceduralMesh|AppendVector2DArray _uvs_2 _uvs ___worldcontext) 0 0 0 0 (ProceduralMesh|AppendProcMeshTangentsArray _tangents _tangents_2 ___worldcontext) false)
          (Class|ProceduralMeshComponent|ClearMeshSection _procedural_mesh _index))))
    (:PreExec
      (bind _triangles_3 (Class|KismetProceduralMeshLibrary|GetSectionfromProceduralMesh _procedural_mesh))
      (LocalVariables|SetNum%20of%20Indices (Utilities|Array|Length _triangles_3)))))

(fn AppendVectorArray
  (params (A :type Array%20of%20Vectors) (B :type Array%20of%20Vectors))
  (Utilities|Array|AppendArray A B)
  (return A))

(fn AppendIntegerArray
  (params (A :type Array%20of%20Integers) (B :type Array%20of%20Integers))
  (Utilities|Array|AppendArray A B)
  (return A))

(fn AppendVector2DArray
  (params (A :type Array%20of%20Vector%202D%20Structures) (B :type Array%20of%20Vector%202D%20Structures))
  (Utilities|Array|AppendArray A B)
  (return A))

(fn AppendProcMeshTangentsArray
  (params (A :type Array%20of%20Proc%20Mesh%20Tangent%20Structures) (B :type Array%20of%20Proc%20Mesh%20Tangent%20Structures))
  (Utilities|Array|AppendArray A B)
  (return A))

(fn RemoveUnusedSections
  (params (Procedural%20Mesh%20Component :type Procedural%20Mesh%20Component%20Object%20Reference))
  (bind (_procedural_mesh _index) (Utilities|ForEachProceduralMeshSection Procedural%20Mesh%20Component)
    (:LoopBody
      (bind _triangles (Class|KismetProceduralMeshLibrary|GetSectionfromProceduralMesh _procedural_mesh _index))
      (if (<= (Utilities|Array|Length _triangles) 0)
        (Class|ProceduralMeshComponent|ClearMeshSection _procedural_mesh _index)))))