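; General-purpose Blueprint function library of small math and utility helpers.
; Math helpers cover normalized XY vector scaling, saturate and one-minus, integer-to-float division, per-axis rotator clamping, negation, and add and subtract.
; FlipBool toggles a bool by reference and returns the result, while the += and -= nodes only return values.
; SetPlayDuration sets a target's play rate to the reciprocal of the duration, which matches that duration only for one-second content.
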(fn VectorXY
  (params (Vector :type Vector) (Scale :type Float%20%28single-precision%29))
  (return (* (Math|Vector|Normalize (Math|Vector|MakeVector (.x Vector) (.y Vector) 0.0)) Scale)))

(fn OneMinus
  (params (in :type Float%20%28single-precision%29))
  (return (- 1.0 (Math|Saturate in (LocalVariables|Get__WorldContext)))))

(fn Saturate
  (params (In :type Float%20%28single-precision%29))
  (return (Math|Float|Clamp(Float) In)))

(fn IntFloatDivision
  (params (A :type Integer) (B :type Integer))
  (return (/ (Math|Conversions|ToFloat(Integer) A) (Math|Conversions|ToFloat(Integer) B))))

(fn ClampRotator
  (params (In :type Rotator) (Min :type Rotator) (Max :type Rotator :default "360.000000,360.000000,360.000000"))
  (return (Math|Rotator|MakeRotator (Math|Float|Clamp(Float) (.roll In) (.roll Min) (.roll Max)) (Math|Float|Clamp(Float) (.pitch In) (.pitch Min) (.pitch Max)) (Math|Float|Clamp(Float) (.yaw In) (.yaw Min) (.yaw Max)))))

(fn +=
  (params (In :type Float%20%28single-precision%29%20%28by%20ref%29) (+ :type Float%20%28single-precision%29))
  (return (+ In +)))

(fn -=
  (params (In :type Float%20%28single-precision%29%20%28by%20ref%29) (- :type Float%20%28single-precision%29))
  (return (- In -)))

(fn Invert
  (params (In :type Float%20%28single-precision%29))
  (return (* In -1.0)))

(fn FlipBool
  (params (In :type Boolean%20%28by%20ref%29))
  (bind _returnvalue (not In))
  (|SetBy-RefVar In _returnvalue)
  (return _returnvalue))

(fn SetPlayDuration
  (params (Target :type Timeline%20Component%20Object%20Reference%20%28by%20ref%29) (New%20Duration :type Float%20%28single-precision%29))
  (Components|Timeline|SetPlayRate Target (/ 1.0 New%20Duration)))