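; Directional light Blueprint that publishes its direction and colour to the Lighting_SPC material parameter collection, so materials can read the scene's light.
; Update writes the actor's forward vector as Light Direction and the light's colour as Light Colour, packing intensity into the alpha channel.
; It runs from the construction script and on BeginPlay, with no per-frame update.
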(event EventBeginPlay
  (CallFunction|Update))

(event EventTick
  (params (DeltaSeconds :type Float%20%28single-precision%29)))

(fn ConstructionScript
  (CallFunction|Update))

(fn Update
  (bind _lightcomponent (Variables|Default|GetLightComponent))
  (bind _returnvalue (Rendering|Components|Light|GetLightColor _lightcomponent))
  (Rendering|Material|SetVectorParameterValue "/Game/Art/Shaders/ParameterCollections/Lighting_SPC.Lighting_SPC" "Light Direction" (Math|Conversions|ToLinearColor(Vector) (Math|Rotator|GetRotationXVector (Transformation|GetActorRotation))) :!class /Script/Engine.KismetMaterialLibrary)
  (Rendering|Material|SetVectorParameterValue "/Game/Art/Shaders/ParameterCollections/Lighting_SPC.Lighting_SPC" "Light Colour" (Utilities|Struct|MakeLinearColor (.r _returnvalue) (.g _returnvalue) (.b _returnvalue) (Variables|/Script/Engine.LightComponentBase|GetIntensity _lightcomponent)) :!class /Script/Engine.KismetMaterialLibrary))