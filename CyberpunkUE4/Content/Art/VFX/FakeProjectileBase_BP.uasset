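; Fake projectile actor that faces a target position and moves toward it by lerping from its spawn location each Tick, without a movement component.
; Sweeping starts off and turns on after a delay, letting blocking hits other than the player pawn end the flight.
; Otherwise an accumulated-time check ends it.
; Destroy only removes the actor, ignoring the hit position; the particle detach and deactivate nodes are unconnected.
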(event Custom|Destroy
  (params (Hit%20Position :type Vector))
  (Actor|DestroyActor))

(event Custom|Initialize
  ;[1 0.374 0] Init initial position
  (bind _output_get (Variables|Default|SetCached%20Position (Transformation|GetActorLocation)))
  (Transformation|SetActorRotation (Math|Conversions|RotationFromXVector (Math|Vector|Normalize (- (Variables|Default|GetTarget%20Position) _output_get))))
  (Variables|Default|SetDuration (/ (Math|Vector|VectorLength (- (Variables|Default|GetTarget%20Position) _output_get)) (Variables|Default|GetSpeed)))
  (Variables|Default|SetSweep false)
  (Utilities|FlowControl|RetriggerableDelay 5.0)
  (Variables|Default|SetSweep true))

(event EventBeginPlay
  (CallFunction|Initialize))

(event EventTick
  (params (DeltaSeconds :type Float%20%28single-precision%29))
  ;[0.5684 1 0.3165] Accumulate timer
  (bind _out (CallFunction|+= (Variables|Default|GetAccumulated%20Time) (* DeltaSeconds (Variables|Default|GetSpeed))))
  ;[0.3521 0.4223 1] Sweep to next position
  (bind _sweephitresult (Transformation|SetActorLocation (Math|Vector|Lerp(Vector) (Variables|Default|GetCached%20Position) (Variables|Default|GetTarget%20Position) (CallFunction|Saturate (/ _out (Variables|Default|GetDuration)))) (Variables|Default|GetSweep) false))
  (if (and (.bblockinghit _sweephitresult) (!= (.hitactor _sweephitresult) (Game|Player|GetPlayerPawn 0))) ; did we hit something along the way?
    (CallFunction|Destroy (.impactpoint _sweephitresult))
    (Development|PrintString "Hello")
    (elif (>= (Variables|Default|GetAccumulated%20Time) (Variables|Default|GetSpeed)) ; or did time run out?
      (CallFunction|Destroy (Variables|Default|GetTarget%20Position)))))

(fn ConstructionScript)