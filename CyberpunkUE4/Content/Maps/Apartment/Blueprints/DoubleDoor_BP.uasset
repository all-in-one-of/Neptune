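; DoubleDoor_BP is a sliding double door that opens when the player pawn enters its trigger box and closes when it leaves.
; A timeline plays or reverses, feeding SetDoorPosition to move both leaves along relative X by a distance derived from each one's bounds.
; The construction script lifts the trigger by its scaled half-height, so its base sits at its parent's origin.
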(event OnComponentBeginOverlap(Trigger)
  (params (OverlappedComponent :type Primitive%20Component%20Object%20Reference) (OtherActor :type Actor%20Object%20Reference) (OtherComp :type Primitive%20Component%20Object%20Reference) (OtherBodyIndex :type Integer) (bFromSweep :type Boolean) (SweepResult :type Hit%20Result%20Structure%20%28by%20ref%29))
  ;[1 1 1] Trigger handling
  (if (== OtherActor (Game|Player|GetPlayerPawn 0))
    (CallFunction|Open)))

(event OnComponentEndOverlap(Trigger)
  (params (OverlappedComponent :type Primitive%20Component%20Object%20Reference) (OtherActor :type Actor%20Object%20Reference) (OtherComp :type Primitive%20Component%20Object%20Reference) (OtherBodyIndex :type Integer))
  ;[1 1 1] Trigger handling
  (if (== OtherActor (Game|Player|GetPlayerPawn 0))
    (CallFunction|Close)))

(event Custom|Close
  (bind _x (Timeline|Animation Reverse)
    (:Update
      (Utilities|FlowControl|Sequence
        (:then_0
          (Utilities|SetDoorPosition (Variables|Default|GetLeftDoor) _x))
        (:then_1
          (Utilities|SetDoorPosition (Variables|Default|GetRightDoor) _x))))))

(event Custom|Open
  (bind _x (Timeline|Animation Play)
    (:Update
      (Utilities|FlowControl|Sequence
        (:then_0
          (Utilities|SetDoorPosition (Variables|Default|GetLeftDoor) _x))
        (:then_1
          (Utilities|SetDoorPosition (Variables|Default|GetRightDoor) _x))))))

(fn ConstructionScript
  (bind _trigger (Variables|Default|GetTrigger))
  (Transformation|SetRelativeLocation _trigger (Math|Vector|MakeVector 0.0 0.0 (.z (Components|Box|GetScaledBoxExtent _trigger))) false false))